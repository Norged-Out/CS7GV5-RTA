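; Manager for a Rock-Paper-Scissors minigame between the player and an NPC, played to a target score.
; SetupRPS creates the score UI and readies the NPC; StartRound rolls a random NPC move, resolves it, plays both animations and updates scores.
; Montage-finished events from both characters unlock the next round or, at game over, trigger victory montage and winner text.
; NPCRef.Lost() fires at game over regardless of winner.
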(event `self.ReceiveBeginPlay`
  (if (not (`self.bSetupDone`))
    (set `self.bSetupDone` true)
    (bind _asbp_pri_player (cast `/Game/Blueprints/BP_Pri_Player` (`GameplayStatics.GetPlayerCharacter` 0)))
    (set `self.PlayerRef` _asbp_pri_player)
    (add `/Game/Blueprints/BP_Pri_Player.OnRPSMontageFinished` (`self.PlayerRef`) (delegate `MontageFinished`))
    (add `/Game/MetaHumans/Girl/BP_Girl.OnRPSMontageFinished` (`self.NPCRef`) (delegate `MontageFinished`))))

(event `MontageFinished`
  (bind _ui (`self.UI`))
  (bind _output_get (set `self.FinishedMontages` (+ (`self.FinishedMontages`) 1)))
  (if (>= _output_get 2)
    (set `self.bRoundActive` false)
    (if (`self.bGameOver`)
      (if (`self.bPlayerWon`)
        (`/Game/Blueprints/BP_Pri_Player.PlayVictoryMontage` (`self.PlayerRef`))
        (`/Game/Blueprints/WBP_RPS.UpdateWinner` _ui "You Won!")
        (else
          (`/Game/MetaHumans/Girl/BP_Girl.PlayVictoryMontage` (`self.NPCRef`))
          (`/Game/Blueprints/WBP_RPS.UpdateWinner` _ui "You Lost!"))))))

(event `SetupRPS`
  (bind _returnvalue (`GameplayStatics.GetPlayerController` 0))
  (`SceneComponent.SetVisibility` (`self.Widget`) false false)
  (`/Engine/EditorBlueprintResources/StandardMacros.IsValid` (`self.UI`)
    (:`Is Not Valid`
      (bind _returnvalue_2 (`|CreateWidget` "/Game/Blueprints/WBP_RPS.WBP_RPS_C"))
      (bind _output_get (set `self.UI` _returnvalue_2))
      (`UserWidget.AddToViewport` _output_get 0)
      (set `PlayerController.bShowMouseCursor` true _returnvalue)
      (`WidgetBlueprintLibrary.SetInputMode_GameAndUIEx` _returnvalue (`self.UI`))
      (`/Game/MetaHumans/Girl/BP_Girl.Ready` (`self.NPCRef`)))))

(event `StartRound`
  (params (PlayerChosenMove :type "/Game/Blueprints/E_Move Enum" :default "NewEnumerator0"))
  (if (`self.bGameOver`)
    _
    (elif (not (`self.bRoundActive`))
      (set `self.bRoundActive` true)
      (set `self.FinishedMontages` 0)
      (bind _output_get (set `self.PlayerMove` PlayerChosenMove))
      (bind _output_get_2 (set `self.NPCMove` (select `int` (`KismetMathLibrary.RandomIntegerInRange` 0 2) :`0` "NewEnumerator0" :`1` "NewEnumerator1" :`2` "NewEnumerator2" :!type "/Game/Blueprints/E_Move Enum")))
      (bind (_presult _nresult) (`self.ResolveRound` _output_get _output_get_2))
      (set `self.PlayerResult` _presult)
      (set `self.NPCResult` _nresult)
      (`/Game/Blueprints/BP_Pri_Player.PlayRPSAnimation` (`self.PlayerRef`) (`self.PlayerMove`) (`self.PlayerResult`))
      (`/Game/MetaHumans/Girl/BP_Girl.PlayRPSAnimation` (`self.NPCRef`) (`self.NPCMove`) (`self.NPCResult`))
      (`self.HandleScoring`)
      (`/Game/Blueprints/WBP_RPS.UpdateScore` (`self.UI`) (`self.PlayerScore`) (`self.NPCScore`)))))

(fn `HandleScoring`
  (bind _maxscore (`self.MaxScore`))
  (if (`|EnumEquality` (`self.PlayerResult`) "NewEnumerator0")
    (bind _output_get (set `self.PlayerScore` (+ (`self.PlayerScore`) 1))))
  (if (>= _output_get _maxscore)
    (set `self.bPlayerWon` true)
    (set `self.bGameOver` true :!label _label)
    (`/Game/MetaHumans/Girl/BP_Girl.Lost` (`self.NPCRef`))
    (else
      (if (`|EnumEquality` (`self.NPCResult`) "NewEnumerator0")
        (bind _output_get_2 (set `self.NPCScore` (+ (`self.NPCScore`) 1))))
      (if (>= _output_get_2 _maxscore)
        (goto _label)))))

(fn `ResolveRound`
  (params (PMove :type "/Game/Blueprints/E_Move Enum" :default "NewEnumerator0") (NMove :type "/Game/Blueprints/E_Move Enum" :default "NewEnumerator0"))
  (returns (PResult :type "/Game/Blueprints/E_Result Enum") (NResult :type "/Game/Blueprints/E_Result Enum"))
  (locals (PM :type "/Game/Blueprints/E_Move Enum" :default "NewEnumerator0") (NM :type "/Game/Blueprints/E_Move Enum" :default "NewEnumerator0"))
  (bind _output_get (set `local.PM` PMove))
  (bind _output_get_2 (set `local.NM` NMove))
  ; Draw Check
  (if (`|EnumEquality` (`local.PM`) (`local.NM`))
    (return "NewEnumerator2" "NewEnumerator2")
    (else
      ; Player Win
      (if (or (and (`|EnumEquality` (`local.PM`) "NewEnumerator0") (`|EnumEquality` (`local.NM`) "NewEnumerator2")) (or (and (`|EnumEquality` (`local.PM`) "NewEnumerator1") (`|EnumEquality` (`local.NM`) "NewEnumerator0")) (and (`|EnumEquality` (`local.PM`) "NewEnumerator2") (`|EnumEquality` (`local.NM`) "NewEnumerator1"))))
        (return "NewEnumerator0" "NewEnumerator1")
        (else
          (return "NewEnumerator1" "NewEnumerator0"))))))

(fn `UserConstructionScript`)